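; Enemy AI character that patrols between two points and dies from player projectile hits.
; Overlapping either patrol point swaps the current target and writes it to the AI Blackboard, though the initial-point setup is disconnected from BeginPlay.
; Projectile hits decrement health; the killing hit spawns an explosion, increments the first-person player's eliminated-target count, triggers its goal check and destroys the enemy.
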(event EventBeginPlay
  ;[1 1 1] Set the first patrol point
)

(event Collision|EventActorBeginOverlap
  (params (OtherActor :type Actor%20Object%20Reference))
  ;[1 1 1] On ActorBeginOverlap check if a patrol point was reached to switch the next patrol point of the AI
  (if (== (Variables|Default|GetPatrolPoint1) OtherActor)
    (Variables|Default|SetCurrentPatrolPoint (Variables|Default|GetPatrolPoint2))
    (Utilities|UpdatePatrolPointBB)
    (elif (== OtherActor (Variables|Default|GetPatrolPoint2))
      (Variables|Default|SetCurrentPatrolPoint (Variables|Default|GetPatrolPoint1))
      (Utilities|UpdatePatrolPointBB))))

(event Collision|EventHit
  (params (MyComp :type Primitive%20Component%20Object%20Reference) (Other :type Actor%20Object%20Reference) (OtherComp :type Primitive%20Component%20Object%20Reference) (bSelfMoved :type Boolean) (HitLocation :type Vector :default "0, 0, 0") (HitNormal :type Vector :default "0, 0, 0") (NormalImpulse :type Vector :default "0, 0, 0") (Hit :type Hit%20Result%20Structure%20%28by%20ref%29))
  ;[1 1 1] OnHit calculate the EnemyHealth & handle character death
  (Utilities|Casting|CastToBP_FirstPersonProjectile Other)
  (if (> (Variables|Default|GetEnemyHealth) 1)
    (Math|Integer|DecrementInt (Variables|Default|GetEnemyHealth))
    (else
      (Game|SpawnActorfromClass "/Game/StarterContent/Blueprints/Blueprint_Effect_Explosion.Blueprint_Effect_Explosion_C" (Transformation|GetActorTransform) "Undefined" "MultiplyWithRoot" 0 0)
      (bind _asbp_first_person_character (Utilities|Casting|CastToBP_FirstPersonCharacter (Game|GetPlayerCharacter 0)))
      (Math|Integer|IncrementInt (Variables|/Game/FirstPerson/Blueprints/BP_FirstPersonCharacter.BP_FirstPersonCharacter_C|GetTargetsEliminated _asbp_first_person_character)
        (:%20%20
          (Default|CheckGoal _asbp_first_person_character)
          (Actor|DestroyActor))))))

(fn ConstructionScript
  (|CallParentFunction))