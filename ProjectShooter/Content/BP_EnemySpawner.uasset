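; BP_EnemySpawner is a placed actor that keeps the level populated with AI enemies up to a maximum count.
; On BeginPlay a looping timer periodically counts all BP_EnemyCharacter actors and spawns another while the count is below MaxEnemies.
; Each spawn picks a random navigable point within a large radius of the spawner and creates the enemy with the BT_EnemyBehavior behavior tree.
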(event Custom|TryToSpawnEnemy
  ;[1 1 1] Try to spawn an enemy by checking if the max enemies spawned is not yet reached
  (bind _outactors (Actor|GetAllActorsOfClass "/Game/BP_EnemyCharacter.BP_EnemyCharacter_C"))
  (if (< (Utilities|Array|Length _outactors) (Variables|Default|GetMaxEnemies))
    (Utilities|SpawnEnemy)))

(event EventBeginPlay
  ;[1 1 1] Set the timer and loop for the TryToSpawnEnemy event
  (Utilities|Time|SetTimerbyEvent (delegate Custom|TryToSpawnEnemy) (Variables|Default|GetSpawnTime) true))

(fn ConstructionScript)